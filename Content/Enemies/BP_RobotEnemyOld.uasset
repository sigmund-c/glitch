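; Robot enemy that takes projectile damage, shows a health bar once hurt, and fires fireballs from its gun while its blackboard flags it as chasing the player.
; Box overlaps cast to several projectile types, feeding TakeDamage for health and hit markers, then TriggerAnimation for impact effects or death with kill popup and respawn through RespawnerActor.
; A separate below-zero check adds collapse sound and sparks.
; A Delay on Tick paces the shooting.
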(event OnEndPlay(DeathEffect)
  (params (Actor :type Actor%20Object%20Reference) (EndPlayReason :type EEndPlayReason%20Enum :default "Destroyed"))
  ;[1 1 1] Bullet hit AI / damge generate to AI
  (Actor|DestroyActor))

(event OnComponentBeginOverlap(Box)
  (params (OverlappedComponent :type Primitive%20Component%20Object%20Reference) (OtherActor :type Actor%20Object%20Reference) (OtherComp :type Primitive%20Component%20Object%20Reference) (OtherBodyIndex :type Integer) (bFromSweep :type Boolean) (SweepResult :type Hit%20Result%20Structure%20%28by%20ref%29))
  (bind _mesh (Variables|Character|GetMesh))
  ;[1 1 1] Bullet hit AI / damge generate to AI
  (Development|PrintString "OW")
  (bind _asmodified_bp_ky_fire_ball (Utilities|Casting|CastToMODIFIED_BP_ky_fireBall OtherActor)
    (:then
      (CallFunction|TakeDamage (Variables|/Game/FirstPersonBP_UPDATED/Blueprints/weapon/MODIFIED_BP_ky_fireBall.MODIFIED_BP_ky_fireBall_C|GetDamage _asmodified_bp_ky_fire_ball))
      (CallFunction|TriggerAnimation (Transformation|GetWorldLocation (Variables|/Game/FirstPersonBP_UPDATED/Blueprints/weapon/MODIFIED_BP_ky_fireBall.MODIFIED_BP_ky_fireBall_C|GetBox _asmodified_bp_ky_fire_ball)) (Transformation|GetActorLocation _asmodified_bp_ky_fire_ball)))
    (:CastFailed
      (bind _asmodified_bp_rocket (Utilities|Casting|CastToMODIFIED_BP_rocket OtherActor)
        (:then
          (CallFunction|TakeDamage (Variables|/Game/FirstPersonBP_UPDATED/Blueprints/weapon/MODIFIED_BP_rocket.MODIFIED_BP_rocket_C|GetDamage _asmodified_bp_rocket))
          (CallFunction|TriggerAnimation (Transformation|GetWorldLocation (Variables|/Game/FirstPersonBP_UPDATED/Blueprints/weapon/MODIFIED_BP_rocket.MODIFIED_BP_rocket_C|GetStaticMesh _asmodified_bp_rocket)) (Transformation|GetActorLocation _asmodified_bp_rocket)))
        (:CastFailed
          (bind _asmodified_bp_sniper_bullet_fast (Utilities|Casting|CastToMODIFIED_BP_sniper_bullet_fast OtherActor)
            (:then
              (CallFunction|TakeDamage (Variables|/Game/FirstPersonBP_UPDATED/Blueprints/weapon/MODIFIED_BP_sniper_bullet_fast.MODIFIED_BP_sniper_bullet_fast_C|GetDamage _asmodified_bp_sniper_bullet_fast))
              (CallFunction|TriggerAnimation (Transformation|GetWorldLocation (Variables|/Game/FirstPersonBP_UPDATED/Blueprints/weapon/MODIFIED_BP_sniper_bullet_fast.MODIFIED_BP_sniper_bullet_fast_C|GetStaticMesh _asmodified_bp_sniper_bullet_fast)) (Transformation|GetActorLocation _asmodified_bp_sniper_bullet_fast)))
            (:CastFailed
              (bind _asfirst_person_projectile (Utilities|Casting|CastToFirstPersonProjectile OtherActor))
              (CallFunction|TakeDamage 0.3)
              (CallFunction|TriggerAnimation (Transformation|GetWorldLocation (Variables|/Game/FirstPersonBP_UPDATED/Blueprints/FirstPersonProjectile.FirstPersonProjectile_C|GetSphere _asfirst_person_projectile)) (Transformation|GetActorLocation))))))))
  (if (< (Variables|Default|GetHealth) 0.0)
    (Utilities|FlowControl|Sequence
      (:then_0
        (Audio|PlaySoundatLocation "/Game/StarterContent/Audio/Collapse01.Collapse01" (Transformation|GetWorldLocation _mesh) "0, 0, 0" 1.0 1.0 0.0 0 0 0))
      (:then_1
        (bind _returnvalue (Game|SpawnActorfromClass "/Game/StarterContent/Blueprints/Blueprint_Effect_Sparks.Blueprint_Effect_Sparks_C" (Transformation|GetWorldTransform _mesh) "Undefined" 0 0))
        (Variables|Default|SetDeathEffect _returnvalue))
      (:then_2
        (Components|DestroyComponent _mesh)))))

(event EventBeginPlay
  ;[1 1 1] Setup
  (AI|Components|Blackboard|SetValueasVector (AI|GetBlackboard self) (Utilities|Name|MakeLiteralName "EnemyStartLocation") (Transformation|GetActorLocation))
  (bind _returnvalue (UserInterface|CreateWidget "/Game/Enemies/HealthBar.HealthBar_C"))
  (bind _output_get (Variables|Default|SetHealthBar _returnvalue))
  (UserInterface|SetWidget (Variables|Default|GetHealthBarWidget) _output_get)
  (Variables|Default|SetTransform (Transformation|GetActorTransform)))

(event EventTick
  (params (DeltaSeconds :type Float%20%28single-precision%29))
  (bind _gun (Variables|Default|Getgun))
  ;[1 1 1] Health Bar Visibility and Update
  (if (< (Variables|Default|GetHealth) 1.0)
    (Rendering|SetVisibility (Variables|Default|GetHealthBarWidget) true false)
    (Variables|/Game/Enemies/HealthBar.HealthBar_C|SetPercent (Variables|Default|GetHealthBar) (Variables|Default|GetHealth)))
  ;[1 1 1] Shoot at player
  (if (ScalableFloat|GetValueasBool (AI|GetBlackboard self) (Utilities|Name|MakeLiteralName "IsChasingPlayer"))
    (Utilities|FlowControl|Delay 1.0)
    (Components|Animation|PlayAnimation _gun 0 false)
    (Game|SpawnActorfromClass "/Game/ThirdPersonBP/Blueprints/dragon/BP_ky_fireBall_modified.BP_ky_fireBall_modified_C" (Transformation|GetSocketTransform _gun "Gun_EndSocket" "RTS_World") "Undefined" 0 0)))

(fn ConstructionScript)

(fn TakeDamage
  (params (Damage :type Float%20%28single-precision%29))
  (bind _returnvalue (UserInterface|CreateWidget "/Game/ThirdPersonBP/Blueprints/HitMarker.HitMarker_C"))
  (UserInterface|Viewport|AddtoViewport _returnvalue 0)
  (if (== Damage 0.0)
    (Variables|Default|SetHealth (- (Variables|Default|GetHealth) 0.1))
    (else
      (Variables|Default|SetHealth (- (Variables|Default|GetHealth) Damage)))))

(fn TriggerAnimation
  (params (WorldLocation :type Vector) (ActorLocation :type Vector))
  (if (<= (Variables|Default|GetHealth) 0.0)
    (Effects|SpawnEmitteratLocation "/Game/InfinityBladeEffects/Effects/FX_Monsters/FX_Monster_Ausar/P_AU_ShieldSlam_AOE.P_AU_ShieldSlam_AOE" (- WorldLocation "0, 0,88.000000") "0, 0, 0" "0.500000,0.500000,0.500000")
    (Default|RespawnEnemy (Variables|Default|GetRespawnerActor) (Utilities|Struct|MakeS_Respawner_RobotEnemy (Variables|Default|GetRespawnTime) (Utilities|GetClass self) (Variables|Default|GetTransform)))
    (Actor|DestroyActor)
    (bind _returnvalue (UserInterface|CreateWidget "/Game/ThirdPersonBP/Blueprints/KillPopup.KillPopup_C"))
    (UserInterface|Viewport|AddtoViewport _returnvalue 0)
    (else
      (Effects|SpawnEmitteratLocation "/Game/InfinityBladeEffects/Effects/FX_Mobile/ICE/combat/P_Impact_Shield.P_Impact_Shield" ActorLocation))))