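; Clippy NPC that shows an interaction prompt when the player is near and steps through its conversations.
; On BeginPlay it caches the NPCDialogue row names matching its NPCName, and box overlaps show or hide the prompt widget.
; DialogueInteract advances the line number and rebuilds the single dialogue widget with the matching conversation and line.
; Without exactly one match, it closes the widget and moves to the next conversation.
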(event OnComponentBeginOverlap(BoxCollision)
  (params (OverlappedComponent :type Primitive%20Component%20Object%20Reference) (OtherActor :type Actor%20Object%20Reference) (OtherComp :type Primitive%20Component%20Object%20Reference) (OtherBodyIndex :type Integer) (bFromSweep :type Boolean) (SweepResult :type Hit%20Result%20Structure%20%28by%20ref%29))
  ;[1 1 1] Show dialogue prompt when player is near NPC
  (Utilities|Casting|CastToFirstPersonCharacter OtherActor)
  (Utilities|IsValid (Variables|Default|GetDialogueWidget)
    (:Is%20Valid
      (Widget|SetVisibility (Variables|Default|GetDialogueWidget) "Visible"))
    (:Is%20Not%20Valid
      (bind _returnvalue (UserInterface|CreateWidget "/Game/MenuContent/Dialogue/DialogueWidget.DialogueWidget_C" (Game|GetPlayerController 0)))
      (Widget|SetVisibility (Variables|/Game/MenuContent/Dialogue/DialogueWidget.DialogueWidget_C|GetPopUp _returnvalue) "Visible")
      (bind _output_get (Variables|Default|SetDialogueWidget _returnvalue))
      (UserInterface|Viewport|AddtoViewport _output_get 1))))

(event OnComponentEndOverlap(BoxCollision)
  (params (OverlappedComponent :type Primitive%20Component%20Object%20Reference) (OtherActor :type Actor%20Object%20Reference) (OtherComp :type Primitive%20Component%20Object%20Reference) (OtherBodyIndex :type Integer))
  (bind _dialoguewidget (Variables|Default|GetDialogueWidget))
  ;[1 1 1] Remove dialogue prompt when player moves away from NPC
  (Utilities|Casting|CastToFirstPersonCharacter OtherActor)
  (Utilities|IsValid _dialoguewidget
    (:Is%20Valid
      (Widget|SetVisibility _dialoguewidget "Hidden"))))

(event EventBeginPlay
  ;[1 1 1] Get all dialogue lines belonging to this NPC
  (bind _outrownames (DataTable|GetDataTableRowNames "/Game/MenuContent/Dialogue/NPCDialogue.NPCDialogue"))
  (for _array_element _outrownames
    (bind _returnvalue (Utilities|GetDataTableRow "/Game/MenuContent/Dialogue/NPCDialogue.NPCDialogue" _array_element)
      (:then
        (if (Utilities|Name|Equal(Name) (.npc_name (Utilities|Struct|BreakNPCDialogueStructure_AllLines _returnvalue)) (Variables|Default|GetNPCName))
          (Utilities|Array|Add (Variables|Default|GetDialogueLines) _array_element))))))

(event EventDialogueInteract
  (Math|Integer|IncrementInt (Variables|Default|GetCurrentLineNum)
    (:%20%20
      (CallFunction|CreateDialogue))))

(fn ConstructionScript)

(fn ResetValues
  (Variables|Default|SetCurrentConvoNum 0)
  (Variables|Default|SetCurrentLineNum 0)
  (Variables|Default|SetCurrentDialogueLine "None"))

(fn CreateDialogue
  (Utilities|IsValid (Variables|Default|GetDialogueWidget) ; ensures that there is only one dialogue widget at any time
    (:Is%20Valid
      (Widget|RemovefromParent (Variables|Default|GetDialogueWidget)) ; delete the previous dialogue widget
      (Variables|Default|SetDialogueWidget 0))
    (:Is%20Not%20Valid
      _))
  (bind _returnvalue (UserInterface|CreateWidget "/Game/MenuContent/Dialogue/DialogueWidget.DialogueWidget_C" (Game|GetPlayerController 0)))
  (Widget|SetVisibility (Variables|/Game/MenuContent/Dialogue/DialogueWidget.DialogueWidget_C|GetDialogueBox _returnvalue) "Visible")
  (bind _output_get (Variables|Default|SetDialogueWidget _returnvalue))
  (UserInterface|Viewport|AddtoViewport _output_get 1)
  (bind _dialogueline (CallFunction|GetDialogueLine))
  (Utilities|IsValid _output_get
    (:Is%20Valid
      (Variables|/Game/MenuContent/Dialogue/DialogueWidget.DialogueWidget_C|SetDialogueText _output_get _dialogueline))))

(fn GetDialogueLine
  (for _array_element (Variables|Default|GetDialogueLines)
    (bind _returnvalue (Utilities|GetDataTableRow "/Game/MenuContent/Dialogue/NPCDialogue.NPCDialogue" _array_element)
      (:then
        (if (and (== (Variables|Default|GetCurrentConvoNum) (.convo_num (Utilities|Struct|BreakNPCDialogueStructure_AllLines _returnvalue))) (== (.line_num (Utilities|Struct|BreakNPCDialogueStructure_AllLines _returnvalue)) (Variables|Default|GetCurrentLineNum)))
          (Utilities|Array|Add (LocalVariables|GetLinesToReturn) (.dialogue (Utilities|Struct|BreakNPCDialogueStructure_AllLines _returnvalue)))))))
  (if (== (Utilities|Array|Length (LocalVariables|GetLinesToReturn)) 1)
    (return (Utilities|Array|Get(acopy) (LocalVariables|GetLinesToReturn)))
    (else
      (Widget|RemovefromParent (Variables|Default|GetDialogueWidget))
      (Variables|Default|SetDialogueWidget 0)
      (Variables|Default|SetCurrentLineNum 0)
      (Math|Integer|IncrementInt (Variables|Default|GetCurrentConvoNum)))))